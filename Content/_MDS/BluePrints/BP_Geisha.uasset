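; BP_Geisha is an AI-controlled enemy that mirrors combat, ability and death state to its blackboard.
; It loads abilities from the Geisha row of DT_G_PhaseInfo, and a looping timer ticks their cooldowns down during combat.
; ActivateAbility shuffles indices to pick one and flags it playing if ready, but always returns failure and never starts a cooldown.
; Death stops AIC_Type3's brain logic.
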(event EventBeginPlay
  (|CallParentFunction)
  (CallFunction|Initialization)
  (能力|SetCombatState false)
  (能力|SetHasAbility false)
  (AI|Components|Blackboard|SetValueasBool (AI|GetBlackboard (Variables|Runtime|GetAI%20Controller)) (Utilities|Name|MakeLiteralName "Strafe") true))

(event Collision|EventActorBeginOverlap
  (params (OtherActor :type Actor%20Object%20Reference))
  (|CallParentFunction OtherActor) ; 此节点被禁用，将不会被调用。\n从引脚连出引线来编译功能。
)

(event EventTick
  (params (DeltaSeconds :type Float%20%28single-precision%29))
  (|CallParentFunction DeltaSeconds) ; 此节点被禁用，将不会被调用。\n从引脚连出引线来编译功能。
)

(fn ConstructionScript
  (|CallParentFunction))

(fn HandleBTDeath
  (|CallParentFunction)
  (bind _asaic_type_3 (Utilities|Casting|CastToAIC_Type3 (AI|GetAIController self)))
  (AI|Components|Blackboard|SetValueasBool (AI|GetBlackboard self) (Utilities|Name|MakeLiteralName "IsDead") true)
  (AI|Logic|StopLogic (Variables|/Script/AIModule.AIController|GetBrainComponent _asaic_type_3) ""))

(fn SetCombatState
  (params (In%20Combat :type Boolean))
  (Utilities|FlowControl|Sequence
    (:then_0
      (if (not (Variables|Default|GetIsDead))
        (Variables|Runtime|GetAI%20Controller
          (:then
            (bind _output_get (Variables|Default|SetisCombating In%20Combat))
            (AI|Components|Blackboard|SetValueasBool (AI|GetBlackboard (Variables|Runtime|GetAI%20Controller)) (Utilities|Name|MakeLiteralName "IsCombating") _output_get))
          (:else
            (Variables|Default|SetisCombating false :!label _label)))
        (else
          (goto _label))))
    (:then_1
      (if (Variables|Default|GetisCombating)
        (Utilities|Time|SetTimerbyFunctionName 0 "ManageCoolDowns" 0.1 true)
        (else
          (Utilities|Time|ClearTimerbyFunctionName 0 "ManageCoolDowns"))))
    (:then_2
      (Default|CallOnCombatStateChange (Variables|Default|GetisCombating)))))

(fn ManageCoolDowns
  ;[0.15 0.15 0.15 0.5] 每过0.1秒，所有成员变量降低0.1
  (for (_array_element _array_index) (Variables|Default|GetAbility%20Cool%20Downs)
    (Utilities|Array|SetArrayElem (Variables|Default|GetAbility%20Cool%20Downs) _array_index (Math|Float|Clamp(Float) (- _array_element 0.1) 0.0 9999.0))))

(fn Initialization
  (bind _ability_cool_downs (Variables|Default|GetAbility%20Cool%20Downs))
  (bind _random_ability_indice (Variables|Default|GetRandom%20Ability%20Indice))
  (Variables|Runtime|SetAI%20Controller (Pawn|GetController self))
  (bind _returnvalue (Utilities|GetDataTableRow "/Game/_MDS/Data/DataTable/DT_G_PhaseInfo.DT_G_PhaseInfo" "Geisha")
    (:then
      (bind _output_get (Variables|Default|SetAbilities (Utilities|Struct|BreakS_G_PhaseInfo _returnvalue)))
      (Utilities|Array|Clear _ability_cool_downs)
      (Utilities|Array|Resize _ability_cool_downs (Utilities|Array|Length _output_get))
      (Utilities|Array|Resize _random_ability_indice (Utilities|Array|Length _output_get))
      (for (_ _array_index) _random_ability_indice
        (Utilities|Array|SetArrayElem (Variables|Default|GetRandom%20Ability%20Indice) _array_index _array_index)))))

(fn SetHasAbility
  (params (Has%20Ability :type Boolean))
  (bind _output_get (Variables|Default|SetHas%20Ability Has%20Ability)) ; 初始状态任何技能都能释放
  (AI|Components|Blackboard|SetValueasBool (AI|GetBlackboard (Variables|Runtime|GetAI%20Controller)) (Utilities|Name|MakeLiteralName "HasAbility") _output_get))

(fn ActivateAbility
  (bind _random_ability_indice (Variables|Default|GetRandom%20Ability%20Indice))
  (if (not (Variables|Default|GetIsDead))
    (Utilities|Array|Shuffle _random_ability_indice)
    (bind _output_get (LocalVariables|SetL_Index (Utilities|Array|Get(acopy) _random_ability_indice)))
    (Variables|运行时|SetCurrent%20Ability%20Info (Utilities|Array|Get(acopy) (Variables|Default|GetAbilities) _output_get))
    (if (== (Utilities|Array|Get(acopy) (Variables|Default|GetAbility%20Cool%20Downs) (LocalVariables|GetL_Index)) 0.0) ; 当前技能冷却时间是否为0
      (能力|SetPlayingAbility true)
      (return false 0.0)
      (else
        (return false 0.0)))))

(fn SetPlayingAbility
  (params (Is%20Playing%20Ability :type Boolean))
  ;[0.15 0.15 0.15 0.5] true:技能结束
  (if (Utilities|Enum|NotEqual(Enum) (Variables|运行时|GetCurrentAction) "NewEnumerator2")
    (if (and (not Is%20Playing%20Ability) (Variables|运行时|GetPlaying%20Ability))
      (Default|CallOnEndAbility (Variables|运行时|GetCurrent%20Ability%20Info)))
    (bind _output_get (Variables|运行时|SetPlaying%20Ability Is%20Playing%20Ability))
    (AI|Components|Blackboard|SetValueasBool (AI|GetBlackboard (Variables|Runtime|GetAI%20Controller)) (Utilities|Name|MakeLiteralName "PlayingAbility") _output_get)
    (if (Variables|运行时|GetPlaying%20Ability)
      (Variables|运行时|SetCurrentAction "NewEnumerator3")
      (else
        (Variables|运行时|SetCurrentAction "NewEnumerator0")))))

(fn GetHasAbility
  (bind _currentaction (Variables|运行时|GetCurrentAction))
  (return (Math|Boolean|ANDBoolean (Variables|Default|GetHas%20Ability) (Utilities|Enum|NotEqual(Enum) _currentaction "NewEnumerator2") (Utilities|Enum|NotEqual(Enum) _currentaction "NewEnumerator1"))))