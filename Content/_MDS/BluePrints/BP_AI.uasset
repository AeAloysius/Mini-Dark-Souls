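; Base AI enemy character that patrols randomly around its spawn, attacks player-faction actors and can be executed from behind.
; Interface events drive rotation toward the target, sphere-overlap damage and slow motion.
; Hits spawn blood, subtract HP, then play a reaction with brief global time-dilation hit-stop, or trigger montage or ragdoll death.
; Executions snap it before the attacker for a montage; HP bar and behavior-tree death functions are empty stubs.
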(event Custom|Random%20Patrol
  ;[0.15 0.15 0.15 0.5] 指定范围内随机点进行巡逻
  (if (Math|Boolean|ANDBoolean (not (Variables|States|GetIsDead)) (Variables|States|GetIsPatrol) (not (Variables|States|GetisCombating))) ; 检查执行巡逻的条件
    (AI|AIMoveTo self (.RandomLocation (AI|Navigation|GetRandomReachablePointinRadius (Variables|Private|GetInitLocation) (Variables|Combat|GetPatrolRadius) 0 0)) 0 5.0 false
      (:OnSuccess
        (Utilities|FlowControl|Delay (Math|Random|RandomFloatinRange 1.0 4.0))
        (if (not (Variables|States|GetisCombating))
          (CallFunction|RandomPatrol))))))

(event EventBeginPlay
  (Variables|Private|SetCurHP (Variables|预设|GetMaxHp))
  (Variables|Private|SetInitLocation (Transformation|GetActorLocation)))

(event Collision|EventActorBeginOverlap
  (params (OtherActor :type Actor%20Object%20Reference)))

(event EventTick
  (params (DeltaSeconds :type Float%20%28single-precision%29))
  ;[0.15 0.15 0.15 0.5] 受击逻辑
)

(event EventINTHitHandle
  (params (DamageCauser :type Actor%20Object%20Reference) (ReceiveDamage :type Float%20%28double-precision%29) (KnockBackPower :type Integer) (AdditionalInfo :type Array%20of%20Strings))
  ;[0.15 0.15 0.15 0.5] 受击逻辑
  (if (not (Variables|States|GetIsDead))
    (Variables|Private|SetDamage%20Causer DamageCauser)
    (Variables|Private|SetReceive%20Damage ReceiveDamage)
    (Variables|Private|SetKnock%20Back%20Power KnockBackPower)
    (Variables|Private|SetAdditional%20Info AdditionalInfo)
    (if (and (not (Variables|States|GetIsRolling)) (not (Variables|States|GetisInvincible)))
      (switch string (Utilities|Array|Get(acopy) (Variables|Private|GetAdditional%20Info))
        (:Default
          (CallFunction|HandleHitVFX))
        (:executed
          _))
      (bind _output_get (Variables|Private|SetCurHP (- (Variables|Private|GetCurHP) (Variables|Private|GetReceive%20Damage))))
      (Overriden|UpdateHPBar _output_get (Variables|预设|GetMaxHp))
      (if (<= _output_get 0.0)
        (if (Variables|States|GetIsDead)
          (if (Utilities|Enum|Equal(Enum) (Utilities|Array|Get(acopy) (Variables|Private|GetAdditional%20Info)) "executed")
            (CallFunction|InvalidCapsules :!label _label))
          (else
            (Variables|States|SetIsDead true)
            (CallFunction|HandleRotation)
            (CallFunction|HandleDeathAction)
            (goto _label)))
        (else
          (bind _output_get_2 (Variables|States|SetIsHitted true))
          (CallFunction|INTSetHeadBarHittedVisibility _output_get_2)
          ;;[0.15 0.15 0.15 0.5] 霸体
          (CallFunction|HandleRotation)
          (CallFunction|HandleHitAnim)
          ;;[0.15 0.15 0.15 0.5] 顿挫，卡肉
          (Utilities|Time|SetGlobalTimeDilation 0.1)
          (Utilities|FlowControl|Delay 0.005)
          (Utilities|Time|SetGlobalTimeDilation 1.0))))))

(event EventINTPlaybeExecuted
  (params (Info :type String) (Causer :type Actor%20Object%20Reference))
  ;[0.15 0.15 0.15 0.5] 处决逻辑
  (bind _returnvalue (CallFunction|HandleExecuted Info Causer Causer))
  (Utilities|FlowControl|Sequence
    (:then_0
      (CallFunction|INTHitHandle (Variables|Private|GetDamage%20Causer) (Variables|预设|GetMaxHp) 0 (Utilities|Array|MakeArray "excuted")))
    (:then_1
      (Utilities|FlowControl|Delay 0.63)
      (CallFunction|HandleHitVFX)
      (Audio|SpawnSoundatLocation "/Game/PolygonFantasyRivals/Wavs/Cue_Hit.Cue_Hit" (Transformation|GetActorLocation) "0, 0, 0" 1.0 1.0 0.0 0 0))))

(event EventINTRotateRM
  (params (Start :type Boolean))
  ;[0.15 0.15 0.15 0.5] 攻击时转向玩家
  (if Start
    (Timeline|TL_LoopingTimer Play
      (:Update
        (Variables|Private|GetTargetActor
          (:then
            (Transformation|SetActorRotation (Math|Rotator|MakeRotator 0.0 0.0 (.yaw (Math|Interpolation|RInterpTo (Transformation|GetActorRotation) (Math|Rotator|FindLookatRotation (Transformation|GetActorLocation) (Transformation|GetActorLocation (Variables|Private|GetTargetActor))) (Utilities|Time|GetWorldDeltaSeconds) 1e+01)))))
          (:else
            (CallFunction|INTRotateRM false)))))
    (else
      (Timeline|TL_LoopingTimer Stop))))

(event EventINTSlowMotion
  (params (InitDilation :type Float%20%28double-precision%29) (DelayTime :type Float%20%28double-precision%29))
  (Variables|Default|SetCustomTimeDilation InitDilation)
  (Utilities|FlowControl|Delay DelayTime)
  (Variables|Default|SetCustomTimeDilation 1.0))

(event EventINTSphereCheck
  (params (CenterDis :type Float%20%28double-precision%29) (SphereRadius :type Float%20%28double-precision%29) (DamageRatio :type Float%20%28double-precision%29) (Additional%20Info :type Array%20of%20Strings))
  ;[0.15 0.15 0.15 0.5] 球形射线检测
  (Variables|Private|SetAdditional%20Info Additional%20Info)
  (Variables|Combat|SetDamage%20Ratio DamageRatio)
  (bind _outactors (Collision|SphereOverlapActors (+ (Transformation|GetActorLocation) (* (Transformation|GetActorForwardVector) CenterDis)) SphereRadius (Utilities|Array|MakeArray "ObjectTypeQuery3") 0 (Utilities|Array|MakeArray self)))
  (for _array_element _outactors
    (if (and (Actor|ActorHasTag _array_element "playerFaction") (not (Utilities|Array|ContainsItem (Variables|Combat|GetDamagedActor) _array_element)))
      (Utilities|Array|AddUnique (Variables|Combat|GetDamagedActor) _array_element)
      (Class|BPICombat|INTHitHandle(Message) _array_element self (* (Variables|Combat|GetBaseDamage) (Variables|Combat|GetDamage%20Ratio)) 0 (Variables|Private|GetAdditional%20Info))))
  (Utilities|Array|Clear (Variables|Combat|GetDamagedActor)))

(fn ConstructionScript)

(fn HandleHitVFX
  (Effects|SpawnEmitteratLocation "/Game/PolygonFantasyRivals/Particles/FX_Blood.FX_Blood" (Transformation|GetActorLocation) (Math|Rotator|MakeRotator 0.0 0.0 (Math|Random|RandomFloatinRange -1.8e+02 1.8e+02))))

(fn UpdateHPBar
  (params (CurHP :type Float%20%28double-precision%29) (MaxHP :type Float%20%28double-precision%29)))

(fn HandleRotation
  (if (Variables|预设|GetRotateWhenHit)
    (Transformation|SetActorRotation (Math|Rotator|MakeRotator 0.0 0.0 (.yaw (Math|Rotator|FindLookatRotation (Transformation|GetActorLocation) (Transformation|GetActorLocation (Variables|Private|GetDamage%20Causer))))))))

(fn HandleHitAnim
  (if (Variables|预设|GetPlay%20Hit%20Anim)
    (bind _hit_anim (Variables|预设|GetHit%20Anim)
      (:then
        (Animation|PlayAnimMontage _hit_anim 1.0 "None"))
      (:else))))

(fn HandleDeathAction
  (if (Variables|预设|GetUse%20Death%20Anim)
    (CallFunction|HandleBTDeath)
    (bind _death_anim (Variables|预设|GetDeath%20Anim)
      (:then
        (Animation|PlayAnimMontage _death_anim 1.0 "None"))
      (:else))
    (else
      (Physics|SetSimulatePhysics (Variables|Character|GetMesh) true))))

(fn HandleExecuted
  (params (Anim%20String :type String) (Causer :type Actor%20Object%20Reference) (Damage%20Causer :type Actor%20Object%20Reference))
  (Variables|Private|SetDamage%20Causer Damage%20Causer)
  (if (not (Variables|States|GetIsDead))
    (Variables|States|SetIsDead true)
    (AI|Navigation|StopMovement (Pawn|GetController))
    (Animation|Montage|MontageStop (Components|SkeletalMesh|GetAnimInstance (Variables|Character|GetMesh)) 0.0 0)
    (Components|Activation|Deactivate (Variables|Character|GetCharacterMovement))
    (switch string Anim%20String
      (:executeBack
        (CallFunction|InvalidCapsules)
        (Transformation|SetActorRotation (Math|Rotator|MakeRotator 0.0 0.0 (.yaw (Transformation|GetActorRotation (Variables|Private|GetDamage%20Causer)))))
        (Transformation|SetActorLocation (+ (Transformation|GetActorLocation (Variables|Private|GetDamage%20Causer)) (* (Transformation|GetActorForwardVector (Variables|Private|GetDamage%20Causer)) 70)) false false)
        (CallFunction|INTRotateRM false)
        (bind _returnvalue (Animation|PlayAnimMontage (Variables|预设|GetBeExecutedAnim) 1.0 "None"))
        (return _returnvalue)))))

(fn HandleBTDeath)

(fn InvalidCapsules
  (bind _charactermovement (Variables|Character|GetCharacterMovement))
  (CallFunction|HandleBTDeath)
  (Collision|SetCollisionResponsetoChannel (Variables|Collision|GetCapsuleComponent) "ECC_Pawn" "ECR_Ignore")
  (Collision|SetCollisionResponsetoChannel (Variables|Collision|GetCapsuleComponent) "ECC_WorldDynamic" "ECR_Ignore")
  ;[0.15 0.15 0.15 0.5] 停止移动，取消tick
  (Components|Movement|StopMovementImmediately _charactermovement)
  (Pawn|Components|CharacterMovement|SetMovementMode _charactermovement "MOVE_None" 0)
  (Actor|Tick|SetActorTickEnabled false))

(fn GetCurrentHP
  (return (Variables|Private|GetCurHP)))

(fn INTGetStatus
  (return (not (Variables|States|GetIsDead)) (Variables|预设|GetIs%20Executable) (Variables|States|GetIsHitted)))