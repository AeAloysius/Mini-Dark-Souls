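; BP_E_Type1 is an enemy Blueprint that patrols, spots player-faction pawns and attacks them in melee.
; PawnSensing sighting disables further sensing and starts a chase loop: AI MoveTo the target, play a random attack montage, wait with random jitter, repeat.
; When the target is no longer alive, it returns to its initial location, re-enables sensing and resumes the parent's random patrol.
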(event OnSeePawn(PawnSensing)
  (params (Pawn :type Pawn%20Object%20Reference))
  (Utilities|IsValid Pawn
    (:Is%20Valid
      (if (Actor|ActorHasTag Pawn "PlayerFaction")
        (Variables|Default|SetTargetPawn Pawn)
        (Variables|Default|SetisCombating true)
        (Class|PawnSensingComponent|SetSensingUpdatesEnabled (Variables|Default|GetPawnSensing) false)
        (if (not (Variables|Default|GetIsDead)) ; 敌人自己是否死亡
          ;[0.15 0.15 0.15 0.5] 移动到合适位置，进行攻击
          (AI|AIMoveTo self "0, 0, 0" (Variables|Default|GetTargetPawn) 1e+02 false
            (:OnSuccess
              (if (not (Variables|Default|GetIsDead))
                ;[0.15 0.15 0.15 0.5] 检查玩家阵营角色是否死亡，死亡则回到巡回状态
                (bind _output_get (Variables|Default|SetTargetActor (Variables|Default|GetTargetPawn)))
                (bind _isalived (Class|BPICombat|INTGetStatus(Message) _output_get))
                (if _isalived
                  (bind _randomatk (CallFunction|Type1RandomATKAnim))
                  (bind _returnvalue (Animation|PlayAnimMontage _randomatk 1.0 "None"))
                  (Utilities|FlowControl|Delay (+ _returnvalue (Math|Random|RandomFloatinRange 0.2 1.2)))
                  (CallFunction|RestartChasing)
                  (else
                    (Variables|Default|SetisCombating false)
                    (AI|AIMoveTo 0 (Variables|Default|GetInitLocation self) 0 5.0 false
                      (:OnSuccess
                        (Class|PawnSensingComponent|SetSensingUpdatesEnabled (Variables|Default|GetPawnSensing) true)
                        (CallFunction|RandomPatrol) ; 调用父类函数
                      ))))))
            (:OnFail
              (Utilities|FlowControl|Delay 1.0)
              (CallFunction|RestartChasing))))))))

(event Custom|Restart%20Chasing
  (if (not (Variables|Default|GetIsDead)) ; 敌人自己是否死亡
    ;[0.15 0.15 0.15 0.5] 移动到合适位置，进行攻击
    (AI|AIMoveTo self "0, 0, 0" (Variables|Default|GetTargetPawn) 1e+02 false
      (:OnSuccess
        (if (not (Variables|Default|GetIsDead))
          ;[0.15 0.15 0.15 0.5] 检查玩家阵营角色是否死亡，死亡则回到巡回状态
          (bind _output_get (Variables|Default|SetTargetActor (Variables|Default|GetTargetPawn)))
          (bind _isalived (Class|BPICombat|INTGetStatus(Message) _output_get))
          (if _isalived
            (bind _randomatk (CallFunction|Type1RandomATKAnim))
            (bind _returnvalue (Animation|PlayAnimMontage _randomatk 1.0 "None"))
            (Utilities|FlowControl|Delay (+ _returnvalue (Math|Random|RandomFloatinRange 0.2 1.2)))
            (CallFunction|RestartChasing)
            (else
              (Variables|Default|SetisCombating false)
              (AI|AIMoveTo 0 (Variables|Default|GetInitLocation self) 0 5.0 false
                (:OnSuccess
                  (Class|PawnSensingComponent|SetSensingUpdatesEnabled (Variables|Default|GetPawnSensing) true)
                  (CallFunction|RandomPatrol) ; 调用父类函数
                ))))))
      (:OnFail
        (Utilities|FlowControl|Delay 1.0)
        (CallFunction|RestartChasing)))))

(event EventBeginPlay
  (|CallParentFunction)
  (CallFunction|RandomPatrol) ; 调用父类函数
)

(event Collision|EventActorBeginOverlap
  (params (OtherActor :type Actor%20Object%20Reference)))

(event EventTick
  (params (DeltaSeconds :type Float%20%28single-precision%29)))

(fn ConstructionScript
  (|CallParentFunction))

(fn Type1RandomATKAnim
  (bind _values (Utilities|Map|Values (Variables|Default|GetATKAnims)))
  (Utilities|Array|Shuffle _values)
  (return (Utilities|Array|Get(acopy) _values)))