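; Hammer enemy Blueprint, driven through an AI controller's Blackboard, that detects player-faction pawns and enters combat.
; When PawnSensing sees a pawn tagged PlayerFaction, it stores that pawn as the target and sets its combat flag.
; It then switches sensing updates off, with no re-enable in this graph, and writes both values to the Blackboard.
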(event OnSeePawn(PawnSensing)
  (params (Pawn :type Pawn%20Object%20Reference))
  (bind _self self)
  (bind _returnvalue (AI|GetAIController _self))
  (bind _returnvalue_2 (AI|GetBlackboard _returnvalue))
  ;[0.15 0.15 0.15 0.5] 感知玩家角色并传递到黑板
  (if (Actor|ActorHasTag Pawn "PlayerFaction")
    (Variables|Default|SetTargetActor Pawn)
    (Variables|Default|SetisCombating true)
    (Class|PawnSensingComponent|SetSensingUpdatesEnabled (Variables|Default|GetPawnSensing) false)
    (AI|Components|Blackboard|SetValueasBool _returnvalue_2 (Utilities|Name|MakeLiteralName "IsCombating") true)
    (AI|Components|Blackboard|SetValueasObject _returnvalue_2 (Utilities|Name|MakeLiteralName "TargetActor") (Variables|Default|GetTargetActor))))

(event EventBeginPlay
  (|CallParentFunction) ; 此节点被禁用，将不会被调用。\n从引脚连出引线来编译功能。
)

(event Collision|EventActorBeginOverlap
  (params (OtherActor :type Actor%20Object%20Reference))
  (|CallParentFunction OtherActor) ; 此节点被禁用，将不会被调用。\n从引脚连出引线来编译功能。
)

(event EventTick
  (params (DeltaSeconds :type Float%20%28single-precision%29))
  (|CallParentFunction DeltaSeconds) ; 此节点被禁用，将不会被调用。\n从引脚连出引线来编译功能。
)

(fn ConstructionScript
  (|CallParentFunction))