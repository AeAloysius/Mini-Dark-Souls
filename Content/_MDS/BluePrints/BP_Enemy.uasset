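; Enemy character Blueprint that shows enemy health through an overhead head bar, or through a named boss bar on screen when IsBOSS is set.
; BeginPlay sets up the matching widget, and the UpdateHPBar override forwards HP changes to it.
; Lock-on interface events toggle the target icon and head bar together.
; Being hit reveals the head bar, then hides it after a three-second delay.
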(event EventBeginPlay
  (|CallParentFunction)
  ;[0.15 0.15 0.15 0.5] 初始化后执行
  (if (not (Variables|Default|GetIsBOSS))
    (bind _asui_head_bar (Utilities|Casting|CastToUI_HeadBar (UserInterface|GetUserWidgetObject (Variables|组件|GetHealthBar))))
    (bind _output_get (Variables|Default|SetUI%20Head%20Bar _asui_head_bar))
    (Default|UpDateHP _output_get (CallFunction|GetCurrentHP) (Variables|Default|GetMaxHp))
    (else
      (bind _returnvalue (UserInterface|CreateWidget "/Game/_MDS/BluePrints/UI/UI_BOSSBar.UI_BOSSBar_C"))
      (bind _output_get_2 (Variables|Default|SetUI_BOSS_Bar _returnvalue))
      (Default|UpdateHP _output_get_2 (CallFunction|GetCurrentHP) (Variables|Default|GetMaxHp))
      (Default|UpdateBOSSName _output_get_2 (Variables|Default|GetBOSSName))
      (UserInterface|Viewport|AddtoViewport (Variables|Default|GetUI_BOSS_Bar) 0))))

(event EventINTSetHeadBarHittedVisibility
  (params (IsHitted :type Boolean))
  ;[0.15 0.15 0.15 0.5] 锁定时显示，非锁定隐藏，死亡时隐藏
  (if IsHitted
    (bind _ui_head_bar (Variables|Default|GetUI%20Head%20Bar)
      (:then
        (Widget|SetVisibility _ui_head_bar "Visible")
        (Utilities|FlowControl|Delay 3.0)
        (bind _ui_head_bar_2 (Variables|Default|GetUI%20Head%20Bar)
          (:then
            (Widget|SetVisibility _ui_head_bar_2 "Hidden")
            (Variables|Default|SetIsHitted false))
          (:else)))
      (:else))))

(event EventINTSetLockonVisibility
  (params (DisplayLockIcon :type Boolean))
  (bind _ui_head_bar (Variables|Default|GetUI%20Head%20Bar))
  ;[0.15 0.15 0.15 0.5] 锁定时显示，非锁定隐藏，死亡时隐藏
  (Rendering|SetVisibility (Variables|组件|GetTargetIcon) DisplayLockIcon false)
  (Utilities|IsValid _ui_head_bar
    (:Is%20Valid
      (Widget|SetVisibility _ui_head_bar (select DisplayLockIcon "Visible" "Hidden")))))

(fn ConstructionScript
  (|CallParentFunction))

(fn UpdateHPBar
  (params (CurHP :type Float%20%28double-precision%29) (MaxHP :type Float%20%28double-precision%29))
  (|CallParentFunction CurHP MaxHP)
  (if (Variables|Default|GetIsBOSS)
    (bind _ui_boss_bar (Variables|Default|GetUI_BOSS_Bar)
      (:then
        (Default|UpdateHP _ui_boss_bar CurHP MaxHP))
      (:else))
    (else
      (bind _ui_head_bar (Variables|Default|GetUI%20Head%20Bar)
        (:then
          (Default|UpDateHP _ui_head_bar CurHP MaxHP))
        (:else)))))