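; Type 3 enemy Blueprint variant that connects the enemy's state to its AI behavior tree through the blackboard.
; On BeginPlay, after the parent logic, it writes the spawn location, death flag and patrol flag to the AI controller's blackboard.
; Its death handler calls the parent, then, if the controller is an AIC_Type3, sets IsDead and stops the brain component's logic.
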(event EventBeginPlay
  (bind _self self)
  (bind _returnvalue (AI|GetAIController _self))
  (bind _returnvalue_2 (AI|GetBlackboard _returnvalue))
  (|CallParentFunction)
  ;[0.15 0.15 0.15 0.5] 初始化
  (AI|Components|Blackboard|SetValueasVector _returnvalue_2 (Utilities|Name|MakeLiteralName "InitLocation") (Transformation|GetActorLocation))
  (AI|Components|Blackboard|SetValueasBool _returnvalue_2 (Utilities|Name|MakeLiteralName "IsDead") (Variables|Default|GetIsDead))
  (AI|Components|Blackboard|SetValueasBool _returnvalue_2 (Utilities|Name|MakeLiteralName "IsPatrolling") (Variables|Default|GetIsPatrol)))

(event Collision|EventActorBeginOverlap
  (params (OtherActor :type Actor%20Object%20Reference))
  (|CallParentFunction OtherActor) ; 此节点被禁用，将不会被调用。\n从引脚连出引线来编译功能。
)

(event EventTick
  (params (DeltaSeconds :type Float%20%28single-precision%29))
  (|CallParentFunction DeltaSeconds) ; 此节点被禁用，将不会被调用。\n从引脚连出引线来编译功能。
)

(fn ConstructionScript
  (|CallParentFunction))

(fn HandleBTDeath
  (|CallParentFunction)
  (bind _asaic_type_3 (Utilities|Casting|CastToAIC_Type3 (AI|GetAIController self)))
  (AI|Components|Blackboard|SetValueasBool (AI|GetBlackboard self) (Utilities|Name|MakeLiteralName "IsDead") true)
  (AI|Logic|StopLogic (Variables|/Script/AIModule.AIController|GetBrainComponent _asaic_type_3) ""))